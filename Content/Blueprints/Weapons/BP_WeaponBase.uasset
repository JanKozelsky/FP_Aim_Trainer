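; Base weapon Blueprint that handles magazine ammo, firing and timed reloading, leaving WeaponTrace empty, apparently for child weapons.
; FireWeapon spends a round, spawns muzzle particles and sound at the Arrow component, calls WeaponTrace, and auto-reloads when the magazine is empty.
; Automatic and manual reloads share a DoOnce gate that shows an animated reload-bar widget, refills after ReloadTime, then resets.
; It also exposes an FOV multiplier getter.
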(event `self.ReceiveBeginPlay`
  ;[0 0 0] Beginplay
  (set `self.Ammo` (`self.MaxMagazineAmmo`)))

(event `WeaponTrace`)

(event `/Game/Blueprints/FirstPersonTemplate/BPI_Weapon.FireWeapon`
  ;[0 0 0] Weapon Fire Logic
  (`/Game/Blueprints/Libraries/BPML_Comparisons.INT<=INT` (`self.Ammo`)
    (:`True`
      (`self.ReloadWeapon`))
    (:`False`
      (set `self.Ammo` (- (`self.Ammo`) 1))
      (`self.Weapon Fire Effects`)
      (`self.WeaponTrace`)
      (`/Game/Blueprints/Libraries/BPML_Comparisons.INT<=INT` (`self.Ammo`)
        (:`True`
          (`self.ReloadWeapon`))))))

(event `ReloadWeapon`
  ;[0 0 0] Reload Weapon
  (`/Engine/EditorBlueprintResources/StandardMacros.DoOnce` false :!label _label
    (:`Completed`
      (bind _returnvalue (`|CreateWidget` "/Game/Blueprints/Weapons/WB_ReloadBar.WB_ReloadBar_C"))
      (`/Game/Blueprints/Weapons/WB_ReloadBar.ReloadAnimation` _returnvalue (`self.ReloadTime`))
      (`UserWidget.AddToViewport` _returnvalue 0)
      (`KismetSystemLibrary.Delay` (`self.ReloadTime`))
      (set `self.Ammo` (`self.MaxMagazineAmmo`))
      (goto _label :!via `Reset`))))

(event `/Game/Blueprints/FirstPersonTemplate/BPI_Weapon.Reload`
  ;[0 0 0] Reload Weapon
  (goto _label))

(fn `GetFOVMultiplier`
  (returns (FOVMultiplier :type "Float (double-precision)"))
  (return (`self.FOVMultiplier`)))

(fn `UserConstructionScript`)

(fn `Weapon Fire Effects`
  (bind (_returnvalue_location _returnvalue_rotation) (`KismetMathLibrary.BreakTransform` (`SceneComponent.K2_GetComponentToWorld` (`self.Arrow`))))
  (`GameplayStatics.SpawnEmitterAtLocation` (`self.WeaponFireEmitter`) _returnvalue_location _returnvalue_rotation (`self.WeaponFireEmitteScale`))
  (`GameplayStatics.SpawnSoundAtLocation` (`self.WeaponFireSound`) _returnvalue_location (struct) 1.0 1.0 0.0 null null)
  (return))